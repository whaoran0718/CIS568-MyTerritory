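; Gameplay player controller that handles dog character respawning and in-game text chat.
; On respawn, the local controller passes its player settings to GamePlay_GM to spawn the chosen character, sets the player name and creates a hidden chat widget.
; Chat messages are relayed to every controller in the game mode's list, and T toggles the window and cursor.
; A save-loading function exists, but its only call is in unconnected logic.
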(event `Respawn Dog On Client`
  (bind _myplayername (break `/Game/Project/Blueprints/AllLevels/PlayerInfo` (`self.PlayerSettings`)))
  (if (`self.IsLocalController`)
    (`self.PassCharacterInfoToServer` (`self.PlayerSettings`))
    (`/Game/Project/Blueprints/PlayerState_GM.SetPlayeName` (cast `/Game/Project/Blueprints/PlayerState_GM` (`self.PlayerState`) :!pure true) _myplayername)
    (`KismetSystemLibrary.PrintString` (`KismetTextLibrary.Conv_TextToString` _myplayername) true true (struct :`R` 1.0 :`B` 0.803619 :`A` 1.0) 10.0)))

(event `self.ReceiveBeginPlay`
  ;[1 1 1] Loads player info and pass it to the server side
)

(event `PassCharacterInfoToServer`
  (params (PlayerSettingsInfo :type "/Game/Project/Blueprints/AllLevels/PlayerInfo Structure"))
  ;[1 1 1] Pass player info to server and ask for respawn character
  (set `self.PlayerSettings` PlayerSettingsInfo)
  (`/Game/Project/Blueprints/GamePlay_GM.RespawnPlayer` (cast `/Game/Project/Blueprints/GamePlay_GM` (`GameplayStatics.GetGameMode`) :!pure true) self (`.MyPlayerCharacter_10_9DB3C9A34845ABE488BD20A9A01920F5` (break `/Game/Project/Blueprints/AllLevels/PlayerInfo` (`self.PlayerSettings`))))
  (`self.SetupChatWindow`))

(event `SetupChatWindow`
  ;[1 1 1] Create Gameplay chat window
  (bind _returnvalue (`|CreateWidget` "/Game/Project/UI/AllLevels/GameplayChat.GameplayChat_C"))
  (bind _output_get (set `self.GameplayChatWB` _returnvalue))
  (`UserWidget.AddToViewport` _output_get 0)
  (`Widget.SetVisibility` (`self.GameplayChatWB`) "Hidden"))

(event `GetChatMessage`
  (params (TextToSend :type Text))
  ;[1 1 1] Handle incoming chat
  (set `self.SendText` TextToSend)
  (set `self.SenderName` (`.MyPlayerName_2_2807AB9544CB396A557B9DBA1AD76365` (break `/Game/Project/Blueprints/AllLevels/PlayerInfo` (`self.PlayerSettings`))))
  (for _array_element (`/Game/Project/Blueprints/GamePlay_GM.AllPlayerControllers` (cast `/Game/Project/Blueprints/GamePlay_GM` (`GameplayStatics.GetGameMode`) :!pure true))
    (bind _asgameplayer_pc (cast `/Game/Project/Blueprints/Gameplay/Gameplayer_PC` _array_element))
    (`self.UpdateChat` _asgameplayer_pc (`self.SendText`) (`self.SenderName`))))

(event `UpdateChat`
  (params (SendText :type Text) (SenderName :type Text))
  ;[1 1 1] Update chat
  (`/Game/Project/UI/AllLevels/ChatWindow.UpdateChatWindow` (`/Game/Project/UI/AllLevels/GameplayChat.GameplayChat` (`self.GameplayChatWB`)) SenderName SendText))

(event `Key|T`
  (params (Key :type "Key Structure"))
  (bind _gameplaychatwb (`self.GameplayChatWB`))
  ;[1 1 1] Show chat window
  (:`Pressed`
    (`/Engine/EditorBlueprintResources/StandardMacros.FlipFlop`
      (:`A`
        (set `self.bShowMouseCursor` true)
        (`Widget.SetVisibility` _gameplaychatwb "Visible")
        (`Widget.SetUserFocus` (`/Game/Project/UI/AllLevels/ChatWindow.ChatEntry` (`/Game/Project/UI/AllLevels/GameplayChat.GameplayChat` (`self.GameplayChatWB`))) self))
      (:`B`
        (set `self.bShowMouseCursor` false)
        (`Widget.SetVisibility` _gameplaychatwb "Hidden")))))

(fn `LoadGame`
  (locals (selected_dog :type Integer))
  (bind _returnvalue (`GameplayStatics.LoadGameFromSlot` (`self.PlayerSettingsSave`)))
  (bind _asplayer_save_game (cast `/Game/Project/Blueprints/AllLevels/PlayerSaveGame` _returnvalue))
  (bind _output_get (set `self.PlayerSettings` (`/Game/Project/Blueprints/AllLevels/PlayerSaveGame.S_PlayerInfo` _asplayer_save_game)))
  (bind (_myplayername _myplayerimage _myplayercharacter) (break `/Game/Project/Blueprints/AllLevels/PlayerInfo` _output_get))
  (if (== _myplayercharacter "/Game/Project/Blueprints/BP_Husky.BP_Husky_C")
    (set `local.selected_dog` 0)
    (else
      (bind _output_get_2 (set `local.selected_dog` 1))))
  (`KismetSystemLibrary.PrintString` (`KismetTextLibrary.Conv_TextToString` (`|FormatText` "Load: {Player name} dog: {id}" _myplayername _output_get_2))))

(fn `UserConstructionScript`)