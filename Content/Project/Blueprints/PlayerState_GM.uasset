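; Player state that holds a player's name, score and progress toward the game's maximum score.
; On BeginPlay it copies the name from the settings of player controller 0, rather than from its owning controller.
; AddScoreOnServer adds to the score, recomputes progress against the GameState_GM maximum, then asks that game state to check for a win.
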(event `self.ReceiveBeginPlay`
  (bind _asgameplayer_pc (cast `/Game/Project/Blueprints/Gameplay/Gameplayer_PC` (`GameplayStatics.GetPlayerController` 0)))
  (set `self.Player Name` (`.MyPlayerName_2_2807AB9544CB396A557B9DBA1AD76365` (break `/Game/Project/Blueprints/AllLevels/PlayerInfo` (`/Game/Project/Blueprints/Gameplay/Gameplayer_PC.PlayerSettings` _asgameplayer_pc)))))

(event `self.ReceiveTick`
  (params (DeltaSeconds :type "Float (single-precision)")))

(event `Add Score On Server`
  (params (Score :type "Float (double-precision)"))
  (bind _output_get (set `self.Player Score` (+ Score (`self.Player Score`))))
  (bind _asgame_state_gm (cast `/Game/Project/Blueprints/GameState_GM` (`GameplayStatics.GetGameState`)))
  (set `self.Progress Percent` (/ _output_get (`/Game/Project/Blueprints/GameState_GM.Max Score` _asgame_state_gm)))
  (`/Game/Project/Blueprints/GameState_GM.Check If Win` _asgame_state_gm))

(fn `UserConstructionScript`)