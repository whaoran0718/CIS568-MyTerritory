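; BP_UrinePool is a scene actor representing a urine pool, built from a static mesh, a decal and a capsule.
; The construction script scales the capsule and decal from the mesh's relative X/Y scale, swapping axes for the decal, so resizing the mesh resizes both.
; A ChangeColor event creates dynamic material instances on the mesh and decal and sets their Color parameter to tint the pool.
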(event `self.ReceiveBeginPlay`)

(event `Change Color`
  (params (Color :type "LinearColor Structure (by ref)"))
  (`|ExecutionSequence`
    (:`then_0`
      (bind _returnvalue (`PrimitiveComponent.CreateDynamicMaterialInstance` (`self.StaticMesh`) 0 "/Game/Project/Materials/M_UrinePool.M_UrinePool" "None"))
      (`MaterialInstanceDynamic.SetVectorParameterValue` _returnvalue "Color" Color))
    (:`then_1`
      (bind _returnvalue_2 (`DecalComponent.CreateDynamicMaterialInstance` (`self.Decal`)))
      (`MaterialInstanceDynamic.SetVectorParameterValue` _returnvalue_2 "Color" Color))))

(fn `UserConstructionScript`
  (bind _x (.x (`SceneComponent.RelativeScale3D` (`self.StaticMesh`))))
  (bind _y (.y (`SceneComponent.RelativeScale3D` (`self.StaticMesh`))))
  (`SceneComponent.SetRelativeScale3D` (`self.Capsule`) (`KismetMathLibrary.MakeVector` _x _y 1.0))
  (`SceneComponent.SetRelativeScale3D` (`self.Decal`) (`KismetMathLibrary.MakeVector` 1.0 _y _x)))