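; Lobby game mode that tracks joining players, manages their pawns and launches the match by server travel to TestMap.
; On login, the server registers each controller with the game instance, gathers PlayerStarts and has the LobbyPC set up its menu and settings.
; Respawning destroys and replaces the pawn with a Husky, then refreshes every client's player list, count and available characters.
; Character swaps similarly spawn and possess the chosen class.
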(event `self.K2_PostLogin`
  (params (NewPlayer :type "PlayerController Object Reference"))
  ;[1 1 1] Initial Setup
  (`/Engine/EditorBlueprintResources/ActorMacros.Switch Has Authority`
    (:`Authority`
      (`KismetArrayLibrary.Array_Add` (`self.AllPlayerControllers`) NewPlayer)
      (`|ExecutionSequence`
        (:`then_0`
          (bind _asgame_info_instance (cast `/Game/Project/Blueprints/AllLevels/GameInfoInstance` (`GameplayStatics.GetGameInstance`)))
          (`/Game/Project/Blueprints/AllLevels/GameInfoInstance.add player` _asgame_info_instance NewPlayer))
        (:`then_1`
          (bind _outactors (`GameplayStatics.GetAllActorsOfClass` "/Script/Engine.PlayerStart"))
          (set `self.SpawnPoints` _outactors)
          (bind _asgame_info_instance_2 (cast `/Game/Project/Blueprints/AllLevels/GameInfoInstance` (`GameplayStatics.GetGameInstance`)))
          (set `self.ServerName` (`/Game/Project/Blueprints/AllLevels/GameInfoInstance.ServerName` _asgame_info_instance_2))
          (set `self.MaxPlayers` (`/Game/Project/Blueprints/AllLevels/GameInfoInstance.MaxPlayers` _asgame_info_instance_2))
          (bind _aslobby_pc (cast `/Game/Project/Blueprints/Lobby/LobbyPC` NewPlayer))
          (`/Game/Project/Blueprints/Lobby/LobbyPC.UpdateLobbySettings` _aslobby_pc "/Game/StarterContent/Textures/T_Brick_Clay_Beveled_M.T_Brick_Clay_Beveled_M" "mapname" "111")
          (`/Game/Project/Blueprints/Lobby/LobbyPC.InitialSetup` _aslobby_pc)
          (`/Game/Project/Blueprints/Lobby/LobbyPC.SetupLobbyMenu` _aslobby_pc (`self.ServerName`))
          (`/Game/Project/Blueprints/Lobby/LobbyPC.Respawn on Lobby Client` _aslobby_pc))))))

(event `RespawnPlayer`
  (params (PlayerController :type "PlayerController Object Reference"))
  (bind _returnvalue (`Controller.K2_GetPawn` PlayerController))
  ;[1 1 1] Spawn the player when arriving the looby menu
  (`/Engine/EditorBlueprintResources/StandardMacros.IsValid` _returnvalue
    (:`Is Valid`
      (`self.K2_DestroyActor` _returnvalue))
    (:`Is Not Valid`
      _))
  (bind _returnvalue_2 (`|SpawnActorFromClass` "/Game/Project/Blueprints/BP_Husky.BP_Husky_C" (`self.GetRandomStart`) "Undefined" "OverrideRootScale" null null))
  (`Controller.Possess` PlayerController _returnvalue_2)
  (`self.EveryoneUpdate`))

(event `EveryoneUpdate`
  (bind _allplayercontrollers (`self.AllPlayerControllers`))
  (bind _output_get (set `self.CurrentPlayers` (`KismetArrayLibrary.Array_Length` (`self.AllPlayerControllers`))))
  (if (> _output_get 0)
    (`|ExecutionSequence`
      (:`then_0`
        (`KismetArrayLibrary.Array_Clear` (`self.ConnectedPlayers`))
        (for _array_element _allplayercontrollers
          (bind _aslobby_pc (cast `/Game/Project/Blueprints/Lobby/LobbyPC` _array_element))
          (`KismetArrayLibrary.Array_Add` (`self.ConnectedPlayers`) (`/Game/Project/Blueprints/Lobby/LobbyPC.PlayerSettings` _aslobby_pc))
          (`/Game/Project/Blueprints/Lobby/LobbyPC.UpdateNumbeOfPlayers` _aslobby_pc (`self.CurrentPlayers`) (`self.MaxPlayers`)))
        (for _array_element_2 _allplayercontrollers
          (bind _aslobby_pc_2 (cast `/Game/Project/Blueprints/Lobby/LobbyPC` _array_element_2))
          (`/Game/Project/Blueprints/Lobby/LobbyPC.AddPlayerInfo` _aslobby_pc_2 (`self.ConnectedPlayers`))
          (`/Game/Project/Blueprints/Lobby/LobbyPC.UpdateAvaliableCharacters` _aslobby_pc_2 (`self.AvailableCharacters`)))
        ;[1 1 1] Todo
        (for _array_element_3 (`self.ConnectedPlayers`)
          _))
      (:`then_1`
        (set `self.CanWeStart?` true)))))

(event `LaunchTheGame`
  ;[1 1 1] Start the game
  (`KismetSystemLibrary.ExecuteConsoleCommand` "servertravel TestMap" (`GameplayStatics.GetPlayerController` 0)))

(event `SwapCharacter`
  (params (CharacterClass :type "Character Class Reference") (PlayerController :type "PlayerController Object Reference") (ChangeStatus :type Boolean))
  (bind _returnvalue (`Controller.K2_GetPawn` PlayerController))
  ;[1 1 1] Swap with new selected character
  (`KismetSystemLibrary.PrintString` (`KismetSystemLibrary.GetClassDisplayName` CharacterClass))
  (if (not ChangeStatus)
    (`/Engine/EditorBlueprintResources/StandardMacros.IsValid` _returnvalue
      (:`Is Valid`
        (`self.K2_DestroyActor` _returnvalue))
      (:`Is Not Valid`
        _))
    (bind _returnvalue_2 (`|SpawnActorFromClass` CharacterClass (`self.GetRandomStart`) "Undefined" "OverrideRootScale" null null))
    (`Controller.Possess` PlayerController _returnvalue_2)))

(event `ServerUpdateGameSettings`
  (params (NewParam :type "PlayerController Object Reference")))

(fn `UserConstructionScript`)